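; BP_AddForce is a physics test actor whose cube is pushed by force and steered by input.
; Each tick it prints the result of a visibility line trace and, on a hit, applies forward acceleration to the cube.
; The trace starts at the actor but ends at the cube's scaled down vector in world space, without adding the actor's location.
; The TurnRate axis adds scaled yaw to the actor's rotation.
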(event `self.ReceiveTick`
  (params (DeltaSeconds :type "Float (single-precision)"))
  (bind _cube (`self.Cube`))
  (bind (_outhit _returnvalue) (`KismetSystemLibrary.LineTraceSingle` (`self.K2_GetActorLocation`) (* (- (0.0 0.0 0.0) (`SceneComponent.GetUpVector` _cube)) 10.0) "TraceTypeQuery1"))
  (`KismetSystemLibrary.PrintText` (`KismetTextLibrary.Conv_BoolToText` _returnvalue))
  (if _returnvalue
    (`PrimitiveComponent.AddForce` _cube (* (`SceneComponent.GetForwardVector` _cube) 1000.0) "None" true)))

(event `InputAxis|TurnRate`
  (params (AxisValue :type "Float (single-precision)"))
  (`self.K2_SetActorRotation` (`KismetMathLibrary.MakeRotator` (.roll (`self.K2_GetActorRotation`)) (.pitch (`self.K2_GetActorRotation`)) (+ (.yaw (`self.K2_GetActorRotation`)) (* AxisValue 4.0)))))

(fn `UserConstructionScript`)