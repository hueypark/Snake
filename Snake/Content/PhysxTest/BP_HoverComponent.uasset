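; BP_HoverComponent is a hover component in a PhysX test folder that pushes a mesh away from the surface beneath it.
; InitComponent supplies the mesh to act on.
; Each tick it line traces along its own down vector, with debug drawing on.
; On a hit, it applies force at its own location along the impact normal, fading linearly from HoverForce to zero over TraceLength, without explicit damping.
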(event `InitComponent`
  (params (MeshComponent :type "StaticMeshComponent Object Reference"))
  (set `self.MeshComponent` MeshComponent))

(event `self.ReceiveTick`
  (params (DeltaSeconds :type "Float (single-precision)"))
  (bind _returnvalue (`self.K2_GetComponentLocation`))
  (bind (_outhit _returnvalue_2) (`KismetSystemLibrary.LineTraceSingle` :`Start` _returnvalue :`End` (+ _returnvalue (* (`self.GetUpVector`) (* (`self.TraceLength`) -1.0))) :`TraceChannel` "TraceTypeQuery1" :`DrawDebugType` "ForOneFrame"))
  (if _returnvalue_2
    (bind (_bblockinghit _binitialoverlap _time _location _impactpoint _normal _impactnormal) (`GameplayStatics.BreakHitResult` _outhit))
    (`PrimitiveComponent.AddForceAtLocation` (`self.MeshComponent`) (* _impactnormal (`KismetMathLibrary.Lerp` (`self.HoverForce`) 0.0 (/ (`KismetMathLibrary.VSize` (- _location (`self.K2_GetComponentLocation`))) (`self.TraceLength`)))) (`self.K2_GetComponentLocation`) "None")))