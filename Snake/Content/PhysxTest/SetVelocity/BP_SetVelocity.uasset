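; BP_SetVelocity is a physics test actor that drives its Cube component forward at constant speed while player input steers it.
; Each tick overwrites the Cube's linear velocity along its forward vector, replacing any existing velocity, including vertical.
; The TurnRate axis adds scaled input to the actor's yaw through SetActorRotation without physics teleport, independent of frame time.
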(event `self.ReceiveTick`
  (params (DeltaSeconds :type "Float (single-precision)"))
  (bind _cube (`self.Cube`))
  (`PrimitiveComponent.SetPhysicsLinearVelocity` _cube (* (`SceneComponent.GetForwardVector` _cube) 500.0) false "None"))

(event `InputAxis|TurnRate`
  (params (AxisValue :type "Float (single-precision)"))
  (`self.K2_SetActorRotation` (`KismetMathLibrary.MakeRotator` (.roll (`self.K2_GetActorRotation`)) (.pitch (`self.K2_GetActorRotation`)) (+ (.yaw (`self.K2_GetActorRotation`)) (* AxisValue 4.0)))))

(fn `UserConstructionScript`)