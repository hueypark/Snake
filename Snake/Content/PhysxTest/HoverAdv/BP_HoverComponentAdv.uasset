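; Hover component prototype in the physics tests that applies roll-based torque to a static mesh passed in through Init.
; Each Tick, GetAxisTorque turns the sign of the mesh's world roll into a fixed unit torque, dropping to zero once X angular velocity reaches a limit in that direction.
; The torque acts only on world X as an acceleration change, so it ignores mass.
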(event `Init`
  (params (StaticMeshComponent :type "StaticMeshComponent Object Reference"))
  (set `self.StaticMeshComponent` StaticMeshComponent))

(event `self.ReceiveTick`
  (params (DeltaSeconds :type "Float (single-precision)"))
  (bind _staticmeshcomponent (`self.StaticMeshComponent`))
  (bind _returnvalue (`PrimitiveComponent.GetPhysicsAngularVelocity` _staticmeshcomponent "None"))
  (`PrimitiveComponent.AddTorque` _staticmeshcomponent (`KismetMathLibrary.MakeVector` (`self.GetAxisTorque` (.roll (`SceneComponent.K2_GetComponentRotation` _staticmeshcomponent)) (.x _returnvalue))) "None" true))

(fn `GetAxisTorque`
  (params (AxisRotator :type "Float (double-precision)") (AxisAngularVelocity :type "Float (double-precision)"))
  (returns (Torque :type "Float (double-precision)"))
  (if (< AxisRotator 0.0)
    (if (> AxisAngularVelocity -50.0)
      (return -1.0)
      (else
        _))
    (elif (< AxisAngularVelocity 50.0)
      (return 1.0)
      (else
        _)))
  (return 0.0))