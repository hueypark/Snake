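; BP_Stabilizer damps excessive spin on a physics-simulated static mesh handed to it through Init.
; Each Tick it reads the mesh's angular velocity and applies a counter-torque as an acceleration change, independent of mass.
; GetAxisTorque works bang-bang per axis: a fixed unit torque against the spin above a speed threshold, zero otherwise.
; It also prints the angular velocity every tick.
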(event `Init`
  (params (StaticMeshComponent :type "StaticMeshComponent Object Reference"))
  (set `self.StaticMeshComponetn` StaticMeshComponent))

(event `self.ReceiveTick`
  (params (DeltaSeconds :type "Float (single-precision)"))
  (bind _returnvalue (`PrimitiveComponent.GetPhysicsAngularVelocity` (`self.StaticMeshComponetn`) "None"))
  (`PrimitiveComponent.AddTorque` (`self.StaticMeshComponetn`) (`KismetMathLibrary.MakeVector` (`self.GetAxisTorque` (.x _returnvalue)) (`self.GetAxisTorque` (.y _returnvalue)) (`self.GetAxisTorque` (.z _returnvalue))) "None" true)
  (`KismetSystemLibrary.PrintString` (`KismetStringLibrary.Conv_VectorToString` _returnvalue)))

(fn `GetAxisTorque`
  (params (AngularVelocity :type "Float (double-precision)"))
  (returns (Torque :type "Float (double-precision)"))
  (if (> (`KismetMathLibrary.Abs` AngularVelocity) 100.0)
    (if (> AngularVelocity 0.0)
      (return -1.0)
      (else
        (return 1.0)))
    (else
      (return 0.0))))