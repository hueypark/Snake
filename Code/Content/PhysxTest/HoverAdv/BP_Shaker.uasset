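; BP_Shaker periodically shakes a physics-driven static mesh in the HoverAdv PhysX test.
; Init stores the target StaticMeshComponent, and Tick counts down a timer that rearms about every ten seconds.
; On each expiry it applies a random X/Y torque as an acceleration change, ignoring mass, with no Z torque, and prints a debug "Shake" message.
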(event `Init`
  (params (StaticMeshComponent :type "StaticMeshComponent Object Reference"))
  (set `self.StaticMeshComponent` StaticMeshComponent))

(event `self.ReceiveTick`
  (params (DeltaSeconds :type "Float (single-precision)"))
  (bind _time (`self.TIme`))
  (if (< _time 0.0)
    (set `self.TIme` (+ (`self.TIme`) 10.0))
    (`PrimitiveComponent.AddTorque` (`self.StaticMeshComponent`) (`KismetMathLibrary.MakeVector` (`self.GetRandomAxisTroque`) (`self.GetRandomAxisTroque`)) "None" true)
    (`KismetSystemLibrary.PrintString` "Shake")
    (else
      (set `self.TIme` (- _time DeltaSeconds)))))

(fn `GetRandomAxisTroque`
  (returns (Torque :type "Float (double-precision)"))
  (return (* (`KismetMathLibrary.RandomFloatInRange` -1.0 1.0) 200.0)))