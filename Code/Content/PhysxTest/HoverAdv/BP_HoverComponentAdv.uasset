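; Hover component that steers a physics-simulated static mesh's roll and pitch with torque, leaving yaw untouched.
; Each tick it maps both tilt angles to target angular velocities, scaled linearly up to a cap.
; The gap between target and current physics angular velocity sets a clamped proportional torque, applied as an acceleration change to the mesh supplied through Init.
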(event `Init`
  (params (StaticMeshComponent :type "StaticMeshComponent Object Reference"))
  (set `self.StaticMeshComponent` StaticMeshComponent))

(event `self.ReceiveTick`
  (params (DeltaSeconds :type "Float (single-precision)"))
  (bind _staticmeshcomponent (`self.StaticMeshComponent`))
  (bind _returnvalue (`PrimitiveComponent.GetPhysicsAngularVelocity` _staticmeshcomponent "None"))
  (`PrimitiveComponent.AddTorque` _staticmeshcomponent (`KismetMathLibrary.MakeVector` (`self.GetAxisTorque` (.roll (`SceneComponent.K2_GetComponentRotation` _staticmeshcomponent)) (.x _returnvalue)) (`self.GetAxisTorque` (.pitch (`SceneComponent.K2_GetComponentRotation` _staticmeshcomponent)) (.y _returnvalue))) "None" true))

(fn `GetAxisTorque`
  (params (AxisRotator :type "Float (double-precision)") (AxisAngularVelocity :type "Float (double-precision)"))
  (returns (Torque :type "Float (double-precision)"))
  (bind _desiredvelocity (`self.GetDesiredAxisVelocity` AxisRotator))
  (bind _returnvalue (< _desiredvelocity AxisAngularVelocity))
  (bind _returnvalue_2 (`KismetMathLibrary.Abs` (- _desiredvelocity AxisAngularVelocity)))
  (bind _returnvalue_3 (`KismetMathLibrary.Lerp` 0.0 1.0 (/ _returnvalue_2 10.0)))
  (if (< _returnvalue_2 10.0)
    (if _returnvalue
      (return (- 0.0 _returnvalue_3))
      (else
        (return _returnvalue_3)))
    (elif _returnvalue
      (return (- 0.0 1.0))
      (else
        (return 1.0)))))

(fn `GetDesiredAxisVelocity`
  (params (AxisRotator :type "Float (double-precision)"))
  (returns (DesiredVelocity :type "Float (double-precision)"))
  (bind _returnvalue (`KismetMathLibrary.Abs` AxisRotator))
  (bind _returnvalue_2 (< AxisRotator 0.0))
  (bind _returnvalue_3 (`KismetMathLibrary.Lerp` 0.0 100.0 (/ _returnvalue 60.0)))
  (if (< _returnvalue 60.0)
    (if _returnvalue_2
      (return (- 0.0 _returnvalue_3))
      (else
        (return _returnvalue_3)))
    (elif _returnvalue_2
      (return (- 0.0 100.0))
      (else
        (return 100.0)))))